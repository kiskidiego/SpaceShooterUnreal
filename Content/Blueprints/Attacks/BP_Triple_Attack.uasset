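; BP_Triple_Attack is an attack Blueprint that fires three projectiles in a horizontal fan from a given spawn transform.
; Attack loops over three indices, rotating the spawn forward vector around world Z in 30-degree steps to aim each shot left, center and right.
; Each projectile is requested from the PoolingManager with the spawn location and scale, and a debug string prints per shot.
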(event EventBeginPlay)

(event EventTick
  (params (DeltaSeconds :type Float%20%28single-precision%29)))

(fn Attack
  (params (ProjectileSpawn :type Transform))
  (for _index (range -1 1)
    (Development|PrintString "Triple attack")
    (Default|SpawnObject (Variables|Default|GetPoolingManager) (Variables|Default|GetProjectile) (Math|Transform|MakeTransform (.location ProjectileSpawn) (Math|Conversions|RotationFromXVector (Math|Vector|RotateVectorAroundAxis (Math|Rotator|GetRotationXVector (.rotation ProjectileSpawn)) (Math|Conversions|ToFloat(Integer) (* _index 30)) "0.000000,0.000000,1.000000")) (.scale ProjectileSpawn)))))