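; Railgun attack for the player character that fires a timed burst of projectiles.
; Attack starts the burst, and Tick spawns one projectile per interval until the set amount is reached, then resets.
; Each shot comes from the pooling manager at the player's current BulletSource, with a small random yaw spread around world Z.
; The transform passed to Attack is overwritten before each spawn, so shots follow the player during the burst.
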(event EventBeginPlay
  (|CallParentFunction)
  (bind _asbp_ss_player_character (Utilities|Casting|CastToBP_SS_PlayerCharacter (Game|GetPlayerCharacter 0)))
  (Variables|Default|SetPlayer _asbp_ss_player_character))

(event EventTick
  (params (DeltaSeconds :type Float%20%28single-precision%29))
  (|CallParentFunction DeltaSeconds)
  (if (Variables|Default|GetAttacking)
    (if (< (Variables|Default|GetProjectilesShot) (Variables|Default|GetProjectileAmount))
      (Variables|Default|SetTimer (- (Variables|Default|GetTimer) DeltaSeconds))
      (if (<= (Variables|Default|GetTimer) 0.0)
        (Variables|Default|SetTimer (Variables|Default|GetTimeBetweenProjectiles))
        (Variables|Default|SetProjectilesShot (+ (Variables|Default|GetProjectilesShot) 1))
        (Variables|Default|SetSourceTransform (Transformation|GetWorldTransform (Variables|/Game/Blueprints/BP_SS_PlayerCharacter.BP_SS_PlayerCharacter_C|GetBulletSource (Variables|Default|GetPlayer))))
        (Default|SpawnObject (Variables|Default|GetPoolingManager) (Variables|Default|GetProjectile) (Math|Transform|MakeTransform (.location (Variables|Default|GetSourceTransform)) (Math|Conversions|RotationFromXVector (Math|Vector|RotateVectorAroundAxis (Math|Rotator|GetRotationXVector (.rotation (Variables|Default|GetSourceTransform))) (Math|Random|RandomFloatinRange -5.0 5.0) "0.000000,0.000000,1.000000")) (.scale (Variables|Default|GetSourceTransform)))))
      (else
        (Variables|Default|SetAttacking false)
        (Variables|Default|SetProjectilesShot 0)))))

(fn Attack
  (params (ProjectileSpawn :type Transform))
  (Variables|Default|SetAttacking true)
  (Variables|Default|SetSourceTransform ProjectileSpawn))