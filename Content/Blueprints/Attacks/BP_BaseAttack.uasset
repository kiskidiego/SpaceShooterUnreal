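; BP_BaseAttack is a base attack Blueprint that fires a projectile at a given spawn transform, limited by a cooldown.
; On BeginPlay it takes the PoolingManager from BP_SS_GameMode, and Tick counts the cooldown down.
; CheckAttack resets the cooldown when it has expired, calls Attack and prints a debug string.
; Attack requests the Projectile class from the pooling manager instead of spawning it directly.
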(event EventTick
  (params (DeltaSeconds :type Float%20%28single-precision%29))
  (if (> (Variables|Default|GetCurrentCooldown) -1e+01)
    (Variables|Default|SetCurrentCooldown (- (Variables|Default|GetCurrentCooldown) DeltaSeconds))))

(event EventBeginPlay
  (bind _asbp_ss_game_mode (Utilities|Casting|CastToBP_SS_GameMode (Game|GetGameMode)))
  (Variables|Default|SetPoolingManager (Variables|/Game/Blueprints/BP_SS_GameMode.BP_SS_GameMode_C|GetPoolingManager _asbp_ss_game_mode)))

(fn CheckAttack
  (params (ProjectileSpawn :type Transform))
  (if (<= (Variables|Default|GetCurrentCooldown) 0.0)
    (Variables|Default|SetCurrentCooldown (Variables|Default|GetCooldown))
    (CallFunction|Attack ProjectileSpawn)
    (Development|PrintString "ATTACKING")))

(fn Attack
  (params (ProjectileSpawn :type Transform))
  (Default|SpawnObject (Variables|Default|GetPoolingManager) (Variables|Default|GetProjectile) ProjectileSpawn))