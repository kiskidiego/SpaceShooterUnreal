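; Base enemy for a score-based shooter that flies along its initial forward vector, shoots, and awards points when killed.
; Each tick it moves with sweep and, when its cooldown expires, fires the child attack component with the lowest cooldown from BulletSource.
; It hands itself to the GameMode's PoolingManager when it passes the X boundary or runs out of lives, restoring lives on death for reuse.
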(event EventBeginPlay
  (bind _asbp_ss_game_mode (Utilities|Casting|CastToBP_SS_GameMode (Game|GetGameMode)))
  (Variables|Default|SetGameMode _asbp_ss_game_mode)
  (Variables|Default|SetPoolingManager (Variables|/Game/Blueprints/BP_SS_GameMode.BP_SS_GameMode_C|GetPoolingManager _asbp_ss_game_mode))
  (Variables|Default|SetMovement (Transformation|GetActorForwardVector)))

(event Collision|EventActorBeginOverlap
  (params (OtherActor :type Actor%20Object%20Reference)))

(event EventTick
  (params (DeltaSeconds :type Float%20%28single-precision%29))
  (if (> (.x (Transformation|GetActorLocation)) -2e+03)
    (CallFunction|Move DeltaSeconds)
    (Variables|Default|SetCurrentCooldown (- (Variables|Default|GetCurrentCooldown) DeltaSeconds))
    (CallFunction|TryShoot)
    (else
      (Default|DestroyEnemy (Variables|Default|GetPoolingManager) self))))

(event EventTakeDamage
  (params (Amount :type Integer))
  (bind _gamemode (Variables|Default|GetGameMode))
  (Variables|Default|SetLives (- (Variables|Default|GetLives) Amount))
  (if (<= (Variables|Default|GetLives) 0)
    (Variables|/Game/Blueprints/BP_SS_GameMode.BP_SS_GameMode_C|SetScore _gamemode (+ (Variables|/Game/Blueprints/BP_SS_GameMode.BP_SS_GameMode_C|GetScore _gamemode) (Variables|Default|GetPointsPerKill)))
    (Variables|Default|SetLives (Variables|Default|GetMaxLives))
    (Default|DestroyEnemy (Variables|Default|GetPoolingManager) self)))

(fn ConstructionScript)

(fn Move
  (params (Delta :type Float%20%28double-precision%29))
  (Transformation|SetActorLocation (+ (* (* Delta (Variables|Default|GetSpeed)) (Variables|Default|GetMovement)) (Transformation|GetActorLocation)) true false))

(fn TryShoot
  (if (<= (Variables|Default|GetCurrentCooldown) 0.0)
    (Variables|Default|SetCurrentCooldown (Variables|Default|GetAttackCooldown))
    (for _array_element (Components|GetChildrenComponents (Variables|Default|GetAttacks) true)
      (bind _asbp_base_attack (Utilities|Casting|CastToBP_BaseAttack _array_element))
      (if (< (Variables|/Game/Blueprints/Attacks/BP_BaseAttack.BP_BaseAttack_C|GetCurrentCooldown _asbp_base_attack) (LocalVariables|GetBestCooldown))
        (LocalVariables|SetBestAttack _asbp_base_attack)
        (LocalVariables|SetBestCooldown (Variables|/Game/Blueprints/Attacks/BP_BaseAttack.BP_BaseAttack_C|GetCurrentCooldown _asbp_base_attack))))
    (Utilities|IsValid (LocalVariables|GetBestAttack)
      (:Is%20Valid
        (Default|CheckAttack (LocalVariables|GetBestAttack) (Transformation|GetWorldTransform (Variables|Default|GetBulletSource)))))))