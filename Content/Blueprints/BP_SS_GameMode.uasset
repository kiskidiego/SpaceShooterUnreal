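; Game mode that runs time-based scoring and difficulty scaling until the player dies.
; BeginPlay caches the player character, enemy spawner and pooling manager.
; Tick accumulates time, awarding points at fixed intervals and updating the player's HUD.
; When score reaches a new level, it shortens the spawner's minimum and maximum spawn times down to clamped floors; PlayerDead sets GameOver, halting scoring.
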(event Custom|PlayerDead
  (Variables|Default|SetGameOver true))

(event EventBeginPlay
  (bind _asbp_ss_player_character (Utilities|Casting|CastToBP_SS_PlayerCharacter (Game|GetPlayerCharacter 0)))
  (Variables|Default|SetPlayer _asbp_ss_player_character)
  (bind _returnvalue (Actor|GetActorOfClass "/Game/Blueprints/BP_Spawner.BP_Spawner_C"))
  (Variables|Default|SetSpawner _returnvalue)
  (bind _returnvalue_2 (Actor|GetActorOfClass "/Game/Blueprints/BP_PoolingManager.BP_PoolingManager_C"))
  (Variables|Default|SetPoolingManager _returnvalue_2))

(event EventTick
  (params (DeltaSeconds :type Float%20%28single-precision%29))
  (CallFunction|HandleScoreIncrease DeltaSeconds))

(fn ConstructionScript)

(fn HandleScoreIncrease
  (params (A :type Float%20%28double-precision%29))
  (bind _spawner (Variables|Default|GetSpawner))
  (if (not (Variables|Default|GetGameOver))
    (bind _output_get (Variables|Default|SetTimer (+ A (Variables|Default|GetTimer))))
    (for _index (range 1 (.ReturnValue (Math|Float|Division(WholeandRemainder) _output_get (Variables|Default|GetSecondsPerIncrement))))
      (bind _output_get_2 (Variables|Default|SetScore (+ (Variables|Default|GetPointsPerIncrement) (Variables|Default|GetScore))))
      (Variables|Default|SetTimer 0.0)
      (Default|UpdateScore (Variables|/Game/Blueprints/BP_SS_PlayerCharacter.BP_SS_PlayerCharacter_C|GetHUD (Variables|Default|GetPlayer)) _output_get_2)
      (if (!= (.ReturnValue (Math|Float|Division(WholeandRemainder) (Math|Conversions|ToFloat(Integer) _output_get_2) (Math|Conversions|ToFloat(Integer) (Variables|Default|GetPointsPerLevel)))) (Variables|Default|GetLevel))
        (Variables|Default|SetLevel (.ReturnValue (Math|Float|Division(WholeandRemainder) (Math|Conversions|ToFloat(Integer) _output_get_2) (Math|Conversions|ToFloat(Integer) (Variables|Default|GetPointsPerLevel)))))
        (Variables|/Game/Blueprints/BP_Spawner.BP_Spawner_C|SetEnemySpawnMaxTime _spawner (Math|Float|Clamp(Float) (- (Variables|/Game/Blueprints/BP_Spawner.BP_Spawner_C|GetEnemySpawnMaxTime _spawner) 0.2) 2.0 (Variables|/Game/Blueprints/BP_Spawner.BP_Spawner_C|GetEnemySpawnMaxTime _spawner)))
        (Variables|/Game/Blueprints/BP_Spawner.BP_Spawner_C|SetEnemySpawnMinTime _spawner (Math|Float|Clamp(Float) (- (Variables|/Game/Blueprints/BP_Spawner.BP_Spawner_C|GetEnemySpawnMinTime _spawner) 0.2) 0.5 (Variables|/Game/Blueprints/BP_Spawner.BP_Spawner_C|GetEnemySpawnMinTime _spawner)))))))