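; Object pool manager actor that recycles projectiles, enemies and weapons instead of destroying and respawning them.
; Each Destroy function hides the actor, disables its tick and collision, and stores it in a per-category array.
; Each Spawn function reactivates and moves the first pooled actor of the exact requested class, spawning a new one only when none is found.
; Only projectiles get a Reset call, whether new or reused.
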(event EventBeginPlay)

(event Collision|EventActorBeginOverlap
  (params (OtherActor :type Actor%20Object%20Reference)))

(event EventTick
  (params (DeltaSeconds :type Float%20%28single-precision%29)))

(fn ConstructionScript)

(fn SpawnProjectile
  (params (ProjectileClass :type BP%20Projectile%20Class%20Reference) (Transform :type Transform))
  (bind _projectiles (Variables|Default|GetProjectiles))
  (if (Utilities|Array|IsEmpty _projectiles)
    (bind _returnvalue (Game|SpawnActorfromClass ProjectileClass Transform "Undefined" "MultiplyWithRoot" 0 0 :!label _label))
    (Default|Reset _returnvalue)
    (return _returnvalue)
    (else
      (bind (_array_element _array_index) (Utilities|Array|ForEachLoopwithBreak _projectiles :!label _label_2)
        (:LoopBody
          (if (== (Utilities|GetClass _array_element) ProjectileClass)
            (LocalVariables|SetFirstValidProjectile _array_element)
            (LocalVariables|SetFirstValidIndex _array_index)
            (goto _label_2 Break)))
        (:Completed
          (Utilities|IsValid (LocalVariables|GetFirstValidProjectile)
            (:Is%20Valid
              (Transformation|SetActorTransform (LocalVariables|GetFirstValidProjectile) Transform)
              (Rendering|SetActorHiddenInGame (LocalVariables|GetFirstValidProjectile) false)
              (Actor|Tick|SetActorTickEnabled (LocalVariables|GetFirstValidProjectile) true)
              (Collision|SetActorEnableCollision (LocalVariables|GetFirstValidProjectile) true)
              (Utilities|Array|RemoveIndex (Variables|Default|GetProjectiles) (LocalVariables|GetFirstValidIndex))
              (Development|PrintString (Utilities|GetClassDisplayName ProjectileClass))
              (Default|Reset (LocalVariables|GetFirstValidProjectile))
              (return (LocalVariables|GetFirstValidProjectile)))
            (:Is%20Not%20Valid
              (goto _label))))))))

(fn DestroyProjectile
  (params (Projectile :type BP%20Projectile%20Object%20Reference))
  (Rendering|SetActorHiddenInGame Projectile true)
  (Actor|Tick|SetActorTickEnabled Projectile)
  (Collision|SetActorEnableCollision Projectile false)
  (Utilities|Array|Add (Variables|Default|GetProjectiles) Projectile))

(fn SpawnEnemy
  (params (EnemyClass :type BP%20SS%20Base%20Enemy%20Class%20Reference) (Transform :type Transform))
  (bind _enemies (Variables|Default|GetEnemies))
  (if (Utilities|Array|IsEmpty _enemies)
    (bind _returnvalue (Game|SpawnActorfromClass EnemyClass Transform "Undefined" "MultiplyWithRoot" 0 0 :!label _label))
    (return _returnvalue)
    (else
      (bind (_array_element _array_index) (Utilities|Array|ForEachLoopwithBreak _enemies :!label _label_2)
        (:LoopBody
          (if (== (Utilities|GetClass _array_element) EnemyClass)
            (LocalVariables|SetFirstValidEnemy _array_element)
            (LocalVariables|SetFirstValidIndex _array_index)
            (goto _label_2 Break)))
        (:Completed
          (Utilities|IsValid (LocalVariables|GetFirstValidEnemy)
            (:Is%20Valid
              (Transformation|SetActorTransform (LocalVariables|GetFirstValidEnemy) Transform)
              (Rendering|SetActorHiddenInGame (LocalVariables|GetFirstValidEnemy) false)
              (Actor|Tick|SetActorTickEnabled (LocalVariables|GetFirstValidEnemy) true)
              (Collision|SetActorEnableCollision (LocalVariables|GetFirstValidEnemy) true)
              (Utilities|Array|RemoveIndex (Variables|Default|GetEnemies) (LocalVariables|GetFirstValidIndex))
              (return (LocalVariables|GetFirstValidEnemy)))
            (:Is%20Not%20Valid
              (goto _label))))))))

(fn DestroyEnemy
  (params (Enemy :type BP%20SS%20Base%20Enemy%20Object%20Reference))
  (Rendering|SetActorHiddenInGame Enemy true)
  (Actor|Tick|SetActorTickEnabled Enemy)
  (Collision|SetActorEnableCollision Enemy false)
  (Utilities|Array|Add (Variables|Default|GetEnemies) Enemy))

(fn SpawnWeapon
  (params (WeaponClass :type BP%20Base%20Weapon%20Class%20Reference) (Transform :type Transform))
  (bind _weapons (Variables|Default|GetWeapons))
  (if (Utilities|Array|IsEmpty _weapons)
    (bind _returnvalue (Game|SpawnActorfromClass WeaponClass Transform "Undefined" "MultiplyWithRoot" 0 0 :!label _label))
    (return _returnvalue)
    (else
      (bind (_array_element _array_index) (Utilities|Array|ForEachLoopwithBreak _weapons :!label _label_2)
        (:LoopBody
          (if (== (Utilities|GetClass _array_element) WeaponClass)
            (LocalVariables|SetFirstValidWeapon _array_element)
            (LocalVariables|SetFirstValidIndex _array_index)
            (goto _label_2 Break)))
        (:Completed
          (Utilities|IsValid (LocalVariables|GetFirstValidWeapon)
            (:Is%20Valid
              (Transformation|SetActorTransform (LocalVariables|GetFirstValidWeapon) Transform)
              (Rendering|SetActorHiddenInGame (LocalVariables|GetFirstValidWeapon) false)
              (Actor|Tick|SetActorTickEnabled (LocalVariables|GetFirstValidWeapon) true)
              (Collision|SetActorEnableCollision (LocalVariables|GetFirstValidWeapon) true)
              (Utilities|Array|RemoveIndex (Variables|Default|GetWeapons) (LocalVariables|GetFirstValidIndex))
              (return (LocalVariables|GetFirstValidWeapon)))
            (:Is%20Not%20Valid
              (goto _label))))))))

(fn DestroyWeapon
  (params (Weapon :type BP%20Base%20Weapon%20Object%20Reference))
  (Rendering|SetActorHiddenInGame Weapon true)
  (Actor|Tick|SetActorTickEnabled Weapon)
  (Collision|SetActorEnableCollision Weapon false)
  (Utilities|Array|Add (Variables|Default|GetWeapons) Weapon))