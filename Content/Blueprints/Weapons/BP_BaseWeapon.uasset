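; Base weapon pickup that travels through the level and grants an attack to the player who touches it.
; Each tick it moves along its forward vector at its Speed until it passes a negative X limit.
; Overlapping a Player-tagged actor adds an Attack component to that actor and passes it the weapon's Projectile.
; Both pickup and passing the limit hand the weapon to the game mode's PoolingManager through DestroyWeapon.
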(event EventBeginPlay
  (bind _asbp_ss_game_mode (Utilities|Casting|CastToBP_SS_GameMode (Game|GetGameMode)))
  (Variables|Default|SetPooling%20Manager (Variables|/Game/Blueprints/BP_SS_GameMode.BP_SS_GameMode_C|GetPoolingManager _asbp_ss_game_mode)))

(event Collision|EventActorBeginOverlap
  (params (OtherActor :type Actor%20Object%20Reference))
  (if (Actor|ActorHasTag OtherActor "Player")
    (bind _returnvalue (Game|AddComponentbyClass OtherActor (Variables|Default|GetAttack) false))
    (Variables|/Game/Blueprints/Attacks/BP_BaseAttack.BP_BaseAttack_C|SetProjectile _returnvalue (Variables|Default|GetProjectile))
    (Default|DestroyWeapon (Variables|Default|GetPooling%20Manager) self)))

(event EventTick
  (params (DeltaSeconds :type Float%20%28single-precision%29))
  (bind _returnvalue (Transformation|GetActorForwardVector))
  (bind _returnvalue_2 (Transformation|GetActorLocation))
  (bind _speed (Variables|Default|GetSpeed))
  (bind _returnvalue_3 (* DeltaSeconds _speed))
  (bind _returnvalue_4 (* _returnvalue _returnvalue_3))
  (bind _returnvalue_5 (+ _returnvalue_2 _returnvalue_4))
  (if (> (.x _returnvalue_5) -2e+03)
    (Transformation|SetActorLocation (Math|Vector|MakeVector (.x _returnvalue_5) (.y _returnvalue_5) (.z _returnvalue_5)) false false)
    (else
      (Default|DestroyWeapon (Variables|Default|GetPooling%20Manager) self))))

(fn ConstructionScript)