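; Spawner actor that periodically places enemies and weapon pickups at random child spawn points.
; Tick counts down separate enemy and weapon timers, each reset to a random interval, and pulls actors from the game mode's PoolingManager.
; A random roll bounded by the game mode's Level selects the enemy class, with a random Y offset.
; Weapons get a fixed Y offset and random Attack and Projectile types.
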(event EventBeginPlay
  (bind _asbp_ss_game_mode (Utilities|Casting|CastToBP_SS_GameMode (Game|GetGameMode)))
  (Variables|Default|SetGameMode _asbp_ss_game_mode))

(event Collision|EventActorBeginOverlap
  (params (OtherActor :type Actor%20Object%20Reference)))

(event EventTick
  (params (DeltaSeconds :type Float%20%28single-precision%29))
  (CallFunction|HandleEnemySpawn DeltaSeconds)
  (CallFunction|HandleWeaponSpawn DeltaSeconds))

(fn ConstructionScript)

(fn HandleWeaponSpawn
  (params (Delta :type Float%20%28double-precision%29))
  (bind _output_get (Variables|Default|SetWeaponSpawnTimer (- (Variables|Default|GetWeaponSpawnTimer) Delta)))
  (if (<= _output_get 0.0)
    (Variables|Default|SetWeaponSpawnTimer (Math|Random|RandomFloatinRange (Variables|Default|GetWeaponSpawnMinTime) (Variables|Default|GetWeaponSpawnMaxTime)))
    (CallFunction|SpawnWeapon)))

(fn HandleEnemySpawn
  (params (Delta :type Float%20%28double-precision%29))
  (bind _output_get (Variables|Default|SetEnemySpawnTimer (- (Variables|Default|GetEnemySpawnTimer) Delta)))
  (if (<= _output_get 0.0)
    (Variables|Default|SetEnemySpawnTimer (Math|Random|RandomFloatinRange (Variables|Default|GetEnemySpawnMinTime) (Variables|Default|GetEnemySpawnMaxTime)))
    (CallFunction|SpawnEnemy)))

(fn SpawnEnemy
  (bind _enemyclass (CallFunction|GetEnemytoSpawn (Math|Random|RandomInteger (Variables|/Game/Blueprints/BP_SS_GameMode.BP_SS_GameMode_C|GetLevel (Variables|Default|GetGameMode)))))
  (bind _actor (Default|SpawnObject (Variables|/Game/Blueprints/BP_SS_GameMode.BP_SS_GameMode_C|GetPoolingManager (Variables|Default|GetGameMode)) _enemyclass (Transformation|GetWorldTransform (.OutItem (Utilities|Array|Random (Components|GetChildrenComponents (Variables|Default|GetSpawnPoints) false))))))
  (bind _asbp_ss_base_enemy (Utilities|Casting|CastToBP_SS_BaseEnemy _actor))
  (Transformation|SetActorLocation _asbp_ss_base_enemy (Math|Vector|MakeVector (.x (Transformation|GetActorLocation _asbp_ss_base_enemy)) (+ (.y (Transformation|GetActorLocation _asbp_ss_base_enemy)) (Math|Random|RandomFloatinRange 0.0 (Variables|Default|GetSpawnVariablity))) (.z (Transformation|GetActorLocation _asbp_ss_base_enemy))) false false)
  (return _asbp_ss_base_enemy))

(fn GetEnemytoSpawn
  (params (Type :type Integer))
  (return (Utilities|Select :Index (Math|Integer|Clamp(Integer) Type 0 (- (Variables|Default|GetEnemyTypeAmount) 1)) :Option%200 "/Game/Blueprints/Enemies/BP_SS_BaseEnemy.BP_SS_BaseEnemy_C" :Option%201 "/Game/Blueprints/Enemies/BP_LateralEnemy.BP_LateralEnemy_C" :Option%202 "/Game/Blueprints/Enemies/BP_TripleAttackEnemy.BP_TripleAttackEnemy_C" :Option%203 "/Game/Blueprints/Enemies/BP_Tank.BP_Tank_C")))

(fn SpawnWeapon
  (bind _actor (Default|SpawnObject (Variables|/Game/Blueprints/BP_SS_GameMode.BP_SS_GameMode_C|GetPoolingManager (Variables|Default|GetGameMode)) "/Game/Blueprints/Weapons/BP_BaseWeapon.BP_BaseWeapon_C" (Transformation|GetWorldTransform (.OutItem (Utilities|Array|Random (Components|GetChildrenComponents (Variables|Default|GetSpawnPoints) false))))))
  (bind _asbp_base_weapon (Utilities|Casting|CastToBP_BaseWeapon _actor))
  (Transformation|SetActorLocation _asbp_base_weapon (Math|Vector|MakeVector (.x (Transformation|GetActorLocation _actor)) (+ (.y (Transformation|GetActorLocation _actor)) (Variables|Default|GetSpawnVariablity)) (.z (Transformation|GetActorLocation _actor))) false false)
  (Variables|/Game/Blueprints/Weapons/BP_BaseWeapon.BP_BaseWeapon_C|SetAttack _asbp_base_weapon (.OutItem (Utilities|Array|Random (Variables|Default|GetAttackTypes))))
  (Variables|/Game/Blueprints/Weapons/BP_BaseWeapon.BP_BaseWeapon_C|SetProjectile _asbp_base_weapon (.OutItem (Utilities|Array|Random (Variables|Default|GetProjectileTypes)))))