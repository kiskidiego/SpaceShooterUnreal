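; BP_Weapon is a pickup Blueprint that gives a weapon's attack capability to the object passed into its Hit function.
; Hit adds an Attack component to that object at runtime, then copies the weapon's Projectile value onto the new component.
; The event graph holds only disabled default events, and the construction script just calls its parent.
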(event EventBeginPlay
  (|CallParentFunction) ; This node is disabled and will not be called.\nDrag off pins to build functionality.
)

(event Collision|EventActorBeginOverlap
  (params (OtherActor :type Actor%20Object%20Reference))
  (|CallParentFunction OtherActor) ; This node is disabled and will not be called.\nDrag off pins to build functionality.
)

(event EventTick
  (params (DeltaSeconds :type Float%20%28single-precision%29))
  (|CallParentFunction DeltaSeconds) ; This node is disabled and will not be called.\nDrag off pins to build functionality.
)

(fn ConstructionScript
  (|CallParentFunction))

(fn Hit
  (params (Object :type Actor%20Object%20Reference))
  (bind _returnvalue (Game|AddComponentbyClass Object (Variables|Default|GetAttack) false))
  (Variables|/Game/Blueprints/Attacks/BP_BaseAttack.BP_BaseAttack_C|SetProjectile _returnvalue (Variables|Default|GetProjectile)))