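; Projectile that travels forward while circling a moving pivot, giving it a swirling flight path.
; BeginPlay and Reset pick a random clockwise or counterclockwise direction and place the pivot one radius ahead of the actor.
; Move advances the pivot along its forward vector and sweeps the actor to a sine/cosine offset in world XY.
; Nothing in this Blueprint calls Move; Tick only forwards to the parent.
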(event EventBeginPlay
  (|CallParentFunction)
  (CallFunction|SetRandomDirection)
  (CallFunction|ResetPivot))

(event Collision|EventActorBeginOverlap
  (params (OtherActor :type Actor%20Object%20Reference))
  (|CallParentFunction OtherActor) ; This node is disabled and will not be called.\nDrag off pins to build functionality.
)

(event EventTick
  (params (DeltaSeconds :type Float%20%28single-precision%29))
  (|CallParentFunction DeltaSeconds))

(event EventReset
  (|CallParentFunction)
  (CallFunction|SetRandomDirection)
  (CallFunction|ResetPivot))

(fn ConstructionScript
  (|CallParentFunction))

(fn Move
  (params (Delta :type Float%20%28single-precision%29))
  (bind _radius (Variables|Default|GetRadius))
  (Variables|Default|SetPivot (Math|Transform|MakeTransform (+ (* (* Delta (Variables|Default|GetSpeed)) (Math|Rotator|GetRotationXVector (.rotation (Variables|Default|GetPivot)))) (.location (Variables|Default|GetPivot))) (.rotation (Variables|Default|GetPivot)) "1.000000,1.000000,1.000000"))
  (bind _output_get (Variables|Default|SetAngle (+ (Variables|Default|GetAngle) (* (* (Variables|Default|GetSwirlSpeed) Delta) (Variables|Default|GetDirection)))))
  (Transformation|SetActorLocation (+ (+ (* (* Delta (Variables|Default|GetSpeed)) (Math|Rotator|GetRotationXVector (.rotation (Variables|Default|GetPivot)))) (.location (Variables|Default|GetPivot))) (Math|Vector|MakeVector (* (Math|Trig|Cos(Radians) _output_get) _radius) (* (Math|Trig|Sin(Radians) _output_get) _radius) 0.0)) true false))

(fn SetRandomDirection
  (if (Math|Random|RandomBool)
    (Variables|Default|SetDirection 1.0)
    (else
      (Variables|Default|SetDirection -1.0))))

(fn ResetPivot
  (bind _returnvalue (Transformation|GetActorTransform))
  (Variables|Default|SetAngle (Math|Trig|GetPI))
  (Variables|Default|SetPivot (Math|Transform|MakeTransform (+ (.location _returnvalue) (* (Math|Rotator|GetRotationXVector (.rotation _returnvalue)) (Variables|Default|GetRadius))) (.rotation _returnvalue) "1.000000,1.000000,1.000000")))