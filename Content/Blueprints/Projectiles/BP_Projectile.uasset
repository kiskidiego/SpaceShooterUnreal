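; Pooled projectile that flies forward at a set speed and damages what it overlaps.
; Tick moves it along its forward vector without sweeping and counts down its lifetime.
; Any overlap applies damage to BP_IDamageable targets, then plays an explosion effect and sound.
; On overlap or expiry it returns itself to the game mode's PoolingManager, and Reset restores its lifetime.
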(event EventBeginPlay)

(event Collision|EventActorBeginOverlap
  (params (OtherActor :type Actor%20Object%20Reference))
  (bind _asbp_idamageable (Utilities|Casting|CastToBP_IDamageable OtherActor)
    (:then
      (Default|TakeDamage _asbp_idamageable (Variables|Default|GetDamage)))
    (:CastFailed
      _))
  (Effects|SpawnEmitteratLocation "/Game/StarterContent/Particles/P_Explosion.P_Explosion" (Transformation|GetActorLocation))
  (Audio|PlaySound2D "/Game/StarterContent/Audio/Explosion01.Explosion01" 1.0 1.0 0.0 0 0)
  (bind _asbp_ss_game_mode (Utilities|Casting|CastToBP_SS_GameMode (Game|GetGameMode)))
  (Default|DestroyObject (Variables|/Game/Blueprints/BP_SS_GameMode.BP_SS_GameMode_C|GetPoolingManager _asbp_ss_game_mode) self))

(event EventTick
  (params (DeltaSeconds :type Float%20%28single-precision%29))
  (CallFunction|Move DeltaSeconds)
  (|CallParentFunction 0.0)
  (bind _output_get (Variables|Default|SetLifetime (- (Variables|Default|GetLifetime) DeltaSeconds)))
  (if (< _output_get 0.0)
    (bind _asbp_ss_game_mode (Utilities|Casting|CastToBP_SS_GameMode (Game|GetGameMode)))
    (Default|DestroyObject (Variables|/Game/Blueprints/BP_SS_GameMode.BP_SS_GameMode_C|GetPoolingManager _asbp_ss_game_mode) self)))

(event EventReset
  (Variables|Default|SetLifetime 1e+01))

(fn ConstructionScript)

(fn Move
  (params (Delta :type Float%20%28single-precision%29))
  (Transformation|SetActorLocation (+ (Transformation|GetActorLocation) (* (Transformation|GetActorForwardVector) (* Delta (Variables|Default|GetSpeed)))) false false))